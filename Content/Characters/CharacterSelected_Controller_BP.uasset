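; Player controller that spawns and possesses the character chosen on character select, either Lioness_BP or ThirdPersonCharacter.
; On BeginPlay it reads the LionessTPC flag from CharSelect_GameInstance, then spawns and possesses the matching pawn at a hard-coded location.
; It also spawns the other character unpossessed at a lower point on the same spot.
; When the lioness is chosen, that second spawn follows a delay marked as a temporary hack.
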(event EventBeginPlay
  (bind _aschar_select_game_instance (Utilities|Casting|CastToCharSelect_GameInstance (Game|GetGameInstance)))
  (if (Variables|/Game/Gameplay/CharSelect_GameInstance.CharSelect_GameInstance_C|GetLioness_TPC _aschar_select_game_instance)
    (bind _returnvalue (Game|SpawnActorfromClass "/Game/Characters/Lioness/Lioness_BP.Lioness_BP_C" (Math|Transform|MakeTransform "-970.000000,1843.000000,642.000000" "0, 0, 0" "1,1,1") "Undefined" 0 0))
    (Pawn|Possess _returnvalue)
    ;[1 0.1941 0.4998] Temporary, klejone na sline
    (Utilities|FlowControl|Delay 3.0)
    (Game|SpawnActorfromClass "/Game/Characters/ThirdPersonCharacter/ThirdPersonCharacter.ThirdPersonCharacter_C" (Math|Transform|MakeTransform "-970.000000,1843.000000,380.000000" "0, 0, 0" "1,1,1") "Undefined" 0 0)
    (else
      (bind _returnvalue_2 (Game|SpawnActorfromClass "/Game/Characters/ThirdPersonCharacter/ThirdPersonCharacter.ThirdPersonCharacter_C" (Math|Transform|MakeTransform "-970.000000,1843.000000,642.000000" "0, 0, 0" "1,1,1") "Undefined" 0 0))
      (Pawn|Possess _returnvalue_2)
      (Game|SpawnActorfromClass "/Game/Characters/Lioness/Lioness_BP.Lioness_BP_C" (Math|Transform|MakeTransform "-970.000000,1843.000000,380.000000" "0, 0, 0" "1,1,1") "Undefined" 0 0))))

(event EventTick
  (params (DeltaSeconds :type Float%20%28single-precision%29)))

(fn ConstructionScript)