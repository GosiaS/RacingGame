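; AI controller that steers a character through an ordered series of target points using a behavior tree.
; BeginPlay loads the starting point from a data table, keyed by index as row name, into the blackboard and runs AiJumping_BT.
; Tick advances the index and blackboard location when the first ThirdPersonCharacter found, a hardcoded lookup, nears the current point.
; Older single-target logic using AiTarget_BP remains disconnected.
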(event EventBeginPlay
  (bind _lptargetpoint (Variables|Default|GetLpTargetPoint))
  (bind _outrownames (DataTable|GetDataTableRowNames "/Game/AI/DataRelated/TargetPointsDataSet.TargetPointsDataSet"))
  (bind _output_get (Variables|Default|SetNumOfTargets (Utilities|Array|Length _outrownames)))
  (bind _blackboardcomponent (Class|AIController|UseBlackboard "/Game/AI/AiJumping_BB.AiJumping_BB"))
  (bind _output_get_2 (Variables|Default|SetCurrentBlackBoard _blackboardcomponent))
  (bind _output_get_3 (Variables|Default|SetTargetPointLpName "TargetPointLp"))
  (Class|BlackboardComponent|SetValueasInt _output_get_2 _output_get_3 _lptargetpoint)
  (bind _output_get_4 (Variables|Default|SetRowName (Utilities|Name|MakeLiteralName (Utilities|String|StringToName (Utilities|String|ToString(Integer) _lptargetpoint)))))
  (bind _returnvalue (Utilities|GetDataTableRow "/Game/AI/DataRelated/TargetPointsDataSet.TargetPointsDataSet" _output_get_4)
    (:then
      (bind _output_get_5 (Variables|Default|SetMoveToPositionVector (.PositionVector (Utilities|Struct|BreakTargetPointsStructure _returnvalue))))
      (bind _output_get_6 (Variables|Default|SetMoveLocationName (Utilities|Name|MakeLiteralName "MoveLocation")))
      (AI|Components|Blackboard|SetValueasVector (Variables|Default|GetCurrentBlackBoard) _output_get_6 _output_get_5)
      (AI|RunBehaviorTree "/Game/AI/AiJumping_BT.AiJumping_BT"))))

(event EventTick
  (params (DeltaSeconds :type Float%20%28single-precision%29))
  ;[1 1 1] HARCODED manekin
  (bind _outactors (Actor|GetAllActorsOfClass "/Game/Characters/ThirdPersonCharacter/ThirdPersonCharacter.ThirdPersonCharacter_C"))
  (if (and (Math|Vector|Equal(Vector) (Transformation|GetActorLocation (Utilities|Array|Get(acopy) _outactors)) (Variables|Default|GetMoveToPositionVector) 1e+02) (< (Variables|Default|GetLpTargetPoint) (Variables|Default|GetNumOfTargets)))
    (Development|PrintString "MIJAM PUNKT")
    (bind _result (Math|Integer|IncrementInt (Variables|Default|GetLpTargetPoint))
      (:%20%20
        (Development|PrintString (Utilities|String|ToString(Integer) _result))
        (bind _output_get (Variables|Default|SetRowName (Utilities|Name|MakeLiteralName (Utilities|String|StringToName (Utilities|String|ToString(Integer) _result)))))
        (bind _returnvalue (Utilities|GetDataTableRow "/Game/AI/DataRelated/TargetPointsDataSet.TargetPointsDataSet" _output_get)
          (:then
            (Variables|Default|SetMoveToPositionVector (.PositionVector (Utilities|Struct|BreakTargetPointsStructure _returnvalue)))
            (Class|BlackboardComponent|SetValueasInt (Variables|Default|GetCurrentBlackBoard) (Variables|Default|GetTargetPointLpName) (Variables|Default|GetLpTargetPoint))
            (AI|Components|Blackboard|SetValueasVector (Variables|Default|GetCurrentBlackBoard) (Variables|Default|GetMoveLocationName) (Variables|Default|GetMoveToPositionVector))))))))

(fn ConstructionScript)